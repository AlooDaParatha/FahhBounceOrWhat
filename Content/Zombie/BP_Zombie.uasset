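; BP_Zombie is a zombie that chases the player by retracing their trail, playing a looping drunk-walk animation from BeginPlay.
; Each Tick it records the player's location as a breadcrumb whenever the player has moved beyond a small distance threshold.
; It steers toward the oldest breadcrumb with movement input, removing it once close.
; Rotation is independent of the path: yaw snaps every frame to face the player's current position.
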(event `self.ReceiveBeginPlay`
  (`SkeletalMeshComponent.PlayAnimation` (`self.Mesh`) "/Game/Zombie/Anims/Drunk_Walk.Drunk_Walk" true))

(event `self.ReceiveTick`
  (params (DeltaSeconds :type "Float (single-precision)"))
  (bind _pathpoints (`self.PathPoints`))
  (bind _returnvalue (`self.K2_GetActorLocation` (`GameplayStatics.GetPlayerCharacter` 0)))
  (bind _returnvalue_2 (`self.K2_GetActorLocation` self))
  (bind _output (`|GetArrayItem` _pathpoints))
  (`self.K2_SetActorRotation` self (`KismetMathLibrary.MakeRotator` 0.0 0.0 (.yaw (`KismetMathLibrary.FindLookAtRotation` _returnvalue_2 _returnvalue))) false)
  (if (> (`KismetMathLibrary.VSize` (- _returnvalue (`self.LastRecorded`))) 40.0)
    (`KismetArrayLibrary.Array_Add` (`self.PathPoints`) _returnvalue)
    (set `self.LastRecorded` _returnvalue))
  (if (> (`KismetArrayLibrary.Array_Length` _pathpoints) 0)
    (`self.AddMovementInput` self (`KismetMathLibrary.Normal` (- _output _returnvalue_2)) 1.0 false)
    (if (< (`KismetMathLibrary.VSize` (- _output _returnvalue_2)) 60.0)
      (`KismetArrayLibrary.Array_Remove` _pathpoints))))

(fn `UserConstructionScript`)